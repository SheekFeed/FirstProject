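; BP_Pawn is a drivable pawn whose static mesh continuously pulses in scale.
; Enhanced Input movement offsets it along local X by input times Speed and yaws it by Y signed by X, so steering inverts in reverse.
; Speed and brake actions increment and decrement Speed, braking only while it is positive.
; Tick calls AddWorldScale, which flips ScaleSpeed past either Y-scale limit; neither motion nor pulsing uses delta time.
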(event `self.ReceiveTick`
  (params (DeltaSeconds :type "Float (single-precision)"))
  (`self.AddWorldScale` self))

(event `EnhancedInput|/Game/Inputs/IA_Speed`
  (params (ActionValue :type Boolean) (ElapsedSeconds :type "Float (double-precision)") (TriggeredSeconds :type "Float (double-precision)") (InputAction :type "InputAction Object Reference" :default "/Game/Inputs/IA_Speed.IA_Speed"))
  (:`Triggered`
    (`/Engine/EditorBlueprintResources/StandardMacros.IncrementFloat` (`self.Speed`))))

(event `EnhancedInput|/Game/Inputs/IA_Movement`
  (params (ActionValue :type "Vector2D Structure") (ElapsedSeconds :type "Float (double-precision)") (TriggeredSeconds :type "Float (double-precision)") (InputAction :type "InputAction Object Reference" :default "/Game/Inputs/IA_Movement.IA_Movement"))
  (:`Triggered`
    (`|ExecutionSequence`
      (:`then_0`
        (`self.K2_AddActorLocalRotation` (`KismetMathLibrary.MakeRotator` 0.0 0.0 (* (`KismetMathLibrary.SignOfFloat` ActionValue_X) ActionValue_Y))))
      (:`then_1`
        (`self.K2_AddActorLocalOffset` (`KismetMathLibrary.MakeVector` (* ActionValue_X (`self.Speed`))))))))

(event `EnhancedInput|/Game/Inputs/IA_Brake`
  (params (ActionValue :type Boolean) (ElapsedSeconds :type "Float (double-precision)") (TriggeredSeconds :type "Float (double-precision)") (InputAction :type "InputAction Object Reference" :default "/Game/Inputs/IA_Brake.IA_Brake"))
  (:`Triggered`
    (if (> (`self.Speed`) 0.0)
      (`/Engine/EditorBlueprintResources/StandardMacros.DecrementFloat` (`self.Speed`)))))

(fn `AddWorldScale`
  (bind (_relativescale3d_x _relativescale3d_y) (`KismetMathLibrary.BreakVector` (`SceneComponent.RelativeScale3D` (`self.StaticMesh`))))
  (bind (_relativescale3d_x_2 _relativescale3d_y_2) (`KismetMathLibrary.BreakVector` (`SceneComponent.RelativeScale3D` (`self.StaticMesh`))))
  (if (> _relativescale3d_y (`self.ScaleUpLimitor`))
    (set `self.ScaleSpeed` (* (`self.ScaleSpeed`) -1.0) :!label _label)
    (elif (< _relativescale3d_y_2 (`self.ScaleBottomLimitor`))
      (goto _label)
      (else
        _)))
  (`SceneComponent.SetRelativeScale3D` (`self.StaticMesh`) (+ (`SceneComponent.RelativeScale3D` (`self.StaticMesh`)) (`self.ScaleSpeed`))))

(fn `UserConstructionScript`)