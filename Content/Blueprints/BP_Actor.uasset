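; BP_Actor is an actor that moves continuously while pulsing its scale up and down.
; Each Tick adds MovementSpeed as an unswept world offset, then calls AddWorldScale, with neither step scaled by delta time.
; AddWorldScale negates ScaleSpeed when Y or Z passes the upper or lower limit, ignoring X, then adds it to the scale.
; A local rotation node using RotationSpeed exists but never runs.
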(event `self.ReceiveBeginPlay`)

(event `self.ReceiveTick`
  (params (DeltaSeconds :type "Float (single-precision)"))
  (`self.K2_AddActorWorldOffset` self (`self.MovementSpeed`) false false)
  (`self.AddWorldScale` self))

(fn `AddWorldScale`
  (bind (_scaleuplimitor_x _scaleuplimitor_y _scaleuplimitor_z) (`KismetMathLibrary.BreakVector` (`self.ScaleUpLimitor`)))
  (bind (_scalebottomlimitor_x _scalebottomlimitor_y _scalebottomlimitor_z) (`KismetMathLibrary.BreakVector` (`self.ScaleBottomLimitor`)))
  (bind (_returnvalue_x _returnvalue_y _returnvalue_z) (`KismetMathLibrary.BreakVector` (`self.GetActorScale3D` self)))
  (bind (_returnvalue_x_2 _returnvalue_y_2 _returnvalue_z_2) (`KismetMathLibrary.BreakVector` (`self.GetActorScale3D` self)))
  (if (or (> _returnvalue_y_2 _scaleuplimitor_y) (> _returnvalue_z_2 _scaleuplimitor_z))
    (set `self.ScaleSpeed` (* (`self.ScaleSpeed`) -1.0) :!label _label)
    (elif (or (< _returnvalue_y _scalebottomlimitor_y) (< _returnvalue_z _scalebottomlimitor_z))
      (goto _label)
      (else
        _)))
  (`self.SetActorScale3D` self (+ (`self.GetActorScale3D` self) (`self.ScaleSpeed`))))

(fn `UserConstructionScript`)